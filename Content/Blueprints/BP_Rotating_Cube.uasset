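; BP_Rotating_Cube is an actor that the player turns around the vertical axis with the Q and E keys.
; Key press and release events set two booleans that Tick reads through a Sequence node.
; While a key is held, Tick lowers the yaw for Q or raises it for E at a frame-rate-independent speed of Angle divided by TurningTime.
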(event EventBeginPlay)

(event Collision|EventActorBeginOverlap
  (params (OtherActor :type Actor%20Object%20Reference)))

(event EventTick
  (params (DeltaSeconds :type Float%20%28single-precision%29))
  (bind _returnvalue (Transformation|GetActorRotation))
  (bind _angle (Variables|Default|GetAngle))
  (bind _turningtime (Variables|Default|GetTurningTime))
  (bind _returnvalue_2 (* DeltaSeconds _angle))
  (bind _returnvalue_3 (/ _returnvalue_2 _turningtime))
  (Utilities|FlowControl|Sequence
    (:then_0
      (if (Variables|Default|GetQ_Pressed)
        (Transformation|SetActorRotation (Math|Rotator|MakeRotator 0.0 0.0 (- (.yaw _returnvalue) _returnvalue_3)))))
    (:then_1
      (if (Variables|Default|GetE_Pressed)
        (Transformation|SetActorRotation (Math|Rotator|MakeRotator 0.0 0.0 (+ (.yaw _returnvalue) _returnvalue_3)))))))

(event Input|KeyboardEvents|Q
  (params (Key :type Key%20Structure :default "None"))
  (:Pressed
    (Variables|Default|SetQ_Pressed true))
  (:Released
    (Variables|Default|SetQ_Pressed false)))

(event Input|KeyboardEvents|E
  (params (Key :type Key%20Structure :default "None"))
  (:Pressed
    (Variables|Default|SetE_Pressed true))
  (:Released
    (Variables|Default|SetE_Pressed false)))

(fn ConstructionScript)